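; A pickup actor for one of three terminal keys that the player collects by pressing Interact inside its trigger.
; Trigger overlap enables input and shows an input prompt widget; leaving disables input and removes the prompt.
; On Interact, the actor's Key01/02/03 flag selects which flag to set on the referenced BPTerminal and which "has key" widget to show.
; It then clears prompts, plays audio, hides the key mesh and destroys itself after a delay.
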(event OnComponentBeginOverlap(Trigger)
  (params (OverlappedComponent :type Primitive%20Component%20Object%20Reference) (OtherActor :type Actor%20Object%20Reference) (OtherComp :type Primitive%20Component%20Object%20Reference) (OtherBodyIndex :type Integer) (bFromSweep :type Boolean) (SweepResult :type Hit%20Result%20Structure%20%28by%20ref%29))
  (bind _returnvalue (Game|GetPlayerController 0))
  (Input|EnableInput _returnvalue)
  (bind _returnvalue_2 (UserInterface|CreateWidget "/Game/Gameplay/W_Input.W_Input_C" _returnvalue))
  (UserInterface|Viewport|AddtoViewport _returnvalue_2 0))

(event OnComponentEndOverlap(Trigger)
  (params (OverlappedComponent :type Primitive%20Component%20Object%20Reference) (OtherActor :type Actor%20Object%20Reference) (OtherComp :type Primitive%20Component%20Object%20Reference) (OtherBodyIndex :type Integer))
  (Input|DisableInput (Game|GetPlayerController 0))
  (bind _foundwidgets (Widget|GetAllWidgetsOfClass "/Game/Gameplay/W_Input.W_Input_C" true))
  (for _array_element _foundwidgets
    (Widget|RemovefromParent _array_element)))

(event Input|ActionEvents|InputActionInteract
  (params (Key :type Key%20Structure :default "None"))
  (bind _returnvalue (Game|GetPlayerController 0))
  (:Pressed
    (if (Variables|Default|GetKey_01)
      (Variables|/Game/Gameplay/BP_Terminal.BP_Terminal_C|SetKey_01 (Variables|Default|GetBP_Terminal) true)
      (bind _returnvalue_2 (UserInterface|CreateWidget "/Game/Gameplay/W_Has_key_main_1st.W_Has_key_main_1st_C" _returnvalue))
      (UserInterface|Viewport|AddtoViewport _returnvalue_2 0)
      (bind _foundwidgets (Widget|GetAllWidgetsOfClass "/Game/Gameplay/W_Input.W_Input_C" true :!label _label))
      (for _array_element _foundwidgets
        (Widget|RemovefromParent _array_element))
      (Audio|Components|Audio|Play (Variables|Default|GetAudio) 0.0)
      (Rendering|SetVisibility (Variables|Default|GetMesh_Key_contanier) false true)
      (Utilities|FlowControl|Delay 2.0)
      (Actor|DestroyActor)
      (elif (Variables|Default|GetKey_02)
        (Variables|/Game/Gameplay/BP_Terminal.BP_Terminal_C|SetKey_02 (Variables|Default|GetBP_Terminal) true)
        (bind _returnvalue_3 (UserInterface|CreateWidget "/Game/Gameplay/W_Has_key_main_2nd.W_Has_key_main_2nd_C" _returnvalue))
        (UserInterface|Viewport|AddtoViewport _returnvalue_3 0)
        (goto _label)
        (elif (Variables|Default|GetKey_03)
          (Variables|/Game/Gameplay/BP_Terminal.BP_Terminal_C|SetKey_03 (Variables|Default|GetBP_Terminal) true)
          (bind _returnvalue_4 (UserInterface|CreateWidget "/Game/Gameplay/W_Has_key_main_3rd.W_Has_key_main_3rd_C" _returnvalue))
          (UserInterface|Viewport|AddtoViewport _returnvalue_4 0)
          (goto _label))))))

(fn ConstructionScript)