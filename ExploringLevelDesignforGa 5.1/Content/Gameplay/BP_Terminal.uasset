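; BP_Terminal is an interactable terminal that reveals a button for each of three keys and opens the main door once all three are present.
; Overlapping its table trigger enables player input and shows an input prompt widget, and leaving reverses both.
; On Interact, each key flag shows its button, hidden at BeginPlay, and removes that key's HUD widget with a short delay.
; With all three flags set, it calls OpenDoor on DoorMain and removes the prompt.
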(event OnComponentBeginOverlap(Trigger_table)
  (params (OverlappedComponent :type Primitive%20Component%20Object%20Reference) (OtherActor :type Actor%20Object%20Reference) (OtherComp :type Primitive%20Component%20Object%20Reference) (OtherBodyIndex :type Integer) (bFromSweep :type Boolean) (SweepResult :type Hit%20Result%20Structure%20%28by%20ref%29))
  (bind _returnvalue (Game|GetPlayerController 0))
  (Input|EnableInput _returnvalue)
  (bind _returnvalue_2 (UserInterface|CreateWidget "/Game/Gameplay/W_Input.W_Input_C" _returnvalue))
  (UserInterface|Viewport|AddtoViewport _returnvalue_2 0))

(event OnComponentEndOverlap(Trigger_table)
  (params (OverlappedComponent :type Primitive%20Component%20Object%20Reference) (OtherActor :type Actor%20Object%20Reference) (OtherComp :type Primitive%20Component%20Object%20Reference) (OtherBodyIndex :type Integer))
  (Input|DisableInput (Game|GetPlayerController 0))
  (Widget|RemovefromParent (stale OnComponentBeginOverlap(Trigger_table) _returnvalue_2)))

(event EventBeginPlay
  (Rendering|SetVisibility (Variables|Default|GetButton_contanier) false true))

(event Input|ActionEvents|InputActionInteract
  (params (Key :type Key%20Structure :default "None"))
  (:Pressed
    (if (Variables|Default|GetKey_01)
      (Rendering|SetVisibility (Variables|Default|GetButton_01) true false)
      (bind _foundwidgets (Widget|GetAllWidgetsOfClass "/Game/Gameplay/W_Has_key_main_1st.W_Has_key_main_1st_C" true))
      (Widget|RemovefromParent _foundwidgets)
      (Utilities|FlowControl|Delay 0.5))
    (if (Variables|Default|GetKey_02)
      (Rendering|SetVisibility (Variables|Default|GetButton_02) true false)
      (bind _foundwidgets_2 (Widget|GetAllWidgetsOfClass "/Game/Gameplay/W_Has_key_main_2nd.W_Has_key_main_2nd_C" true))
      (Widget|RemovefromParent _foundwidgets_2)
      (Utilities|FlowControl|Delay 0.5))
    (if (Variables|Default|GetKey_03)
      (Rendering|SetVisibility (Variables|Default|GetButton_03) true false)
      (bind _foundwidgets_3 (Widget|GetAllWidgetsOfClass "/Game/Gameplay/W_Has_key_main_3rd.W_Has_key_main_3rd_C" true))
      (Widget|RemovefromParent _foundwidgets_3)
      (Utilities|FlowControl|Delay 0.5))
    (if (Variables|Default|GetKey_01)
      (if (Variables|Default|GetKey_02)
        (if (Variables|Default|GetKey_03)
          (Default|OpenDoor (Variables|Default|GetDoor_main))
          (Widget|RemovefromParent (stale OnComponentBeginOverlap(Trigger_table) _returnvalue_2)))))))

(fn ConstructionScript)