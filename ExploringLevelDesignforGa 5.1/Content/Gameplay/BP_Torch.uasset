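; BP_Torch is an interactable torch that can be lit once.
; Any overlap with its Box while unlit enables player 0 input and shows a W_Input widget.
; Pressing Interact sets Open, makes LightConteiner and its children visible, then disables input and removes the widget.
; Leaving the Box runs the same cleanup, and the Open flag blocks further prompts once lit.
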(event OnComponentBeginOverlap(Box)
  (params (OverlappedComponent :type Primitive%20Component%20Object%20Reference) (OtherActor :type Actor%20Object%20Reference) (OtherComp :type Primitive%20Component%20Object%20Reference) (OtherBodyIndex :type Integer) (bFromSweep :type Boolean) (SweepResult :type Hit%20Result%20Structure%20%28by%20ref%29))
  (bind _returnvalue (Game|GetPlayerController 0))
  (if (not (Variables|Default|Getopen))
    (Input|EnableInput _returnvalue)
    (bind _returnvalue_2 (UserInterface|CreateWidget "/Game/Gameplay/W_Input.W_Input_C" _returnvalue))
    (UserInterface|Viewport|AddtoViewport _returnvalue_2 0)))

(event OnComponentEndOverlap(Box)
  (params (OverlappedComponent :type Primitive%20Component%20Object%20Reference) (OtherActor :type Actor%20Object%20Reference) (OtherComp :type Primitive%20Component%20Object%20Reference) (OtherBodyIndex :type Integer))
  (Input|DisableInput (Game|GetPlayerController 0))
  (Widget|RemovefromParent (stale OnComponentBeginOverlap(Box) _returnvalue_2)))

(event Input|ActionEvents|InputActionInteract
  (params (Key :type Key%20Structure :default "None"))
  (:Pressed
    (Variables|Default|Setopen true)
    (Rendering|SetVisibility (Variables|Default|GetLight%20conteiner) true true)
    (Input|DisableInput (Game|GetPlayerController 0))
    (Widget|RemovefromParent (stale OnComponentBeginOverlap(Box) _returnvalue_2))))

(fn ConstructionScript)