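; Interactable door actor that opens once, either sliding along local X or rotating to a set yaw.
; Overlapping its box while unopened enables player input and shows a W_Input prompt widget; leaving disables input and removes it.
; Despite its name, the Close event sets Open, animates the door with MoveComponentTo, then runs the same input and prompt cleanup.
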(event OnComponentBeginOverlap(Box)
  (params (OverlappedComponent :type Primitive%20Component%20Object%20Reference) (OtherActor :type Actor%20Object%20Reference) (OtherComp :type Primitive%20Component%20Object%20Reference) (OtherBodyIndex :type Integer) (bFromSweep :type Boolean) (SweepResult :type Hit%20Result%20Structure%20%28by%20ref%29))
  (bind _returnvalue (Game|GetPlayerController 0))
  (if (not (Variables|Default|GetOpen))
    (Input|EnableInput _returnvalue)
    (bind _returnvalue_2 (UserInterface|CreateWidget "/Game/Gameplay/W_Input.W_Input_C" _returnvalue))
    (UserInterface|Viewport|AddtoViewport _returnvalue_2 0)))

(event OnComponentEndOverlap(Box)
  (params (OverlappedComponent :type Primitive%20Component%20Object%20Reference) (OtherActor :type Actor%20Object%20Reference) (OtherComp :type Primitive%20Component%20Object%20Reference) (OtherBodyIndex :type Integer))
  (Input|DisableInput (Game|GetPlayerController 0))
  (Widget|RemovefromParent (stale OnComponentBeginOverlap(Box) _returnvalue_2)))

(event Custom|Close
  (bind _door_rotation_sm (Variables|Default|GetDoor_rotation_sm))
  (bind _door_rotation_sm_2 (Variables|Default|GetDoor_rotation_sm))
  (bind _relativelocation (Variables|/Script/Engine.SceneComponent|GetRelativeLocation _door_rotation_sm))
  (Variables|Default|SetOpen true)
  (if (Variables|Default|Getslide_rotation)
    (Components|MoveComponentTo _door_rotation_sm (Math|Vector|MakeVector (+ (.x _relativelocation) (Variables|Default|Getslide_lenght)) (.y _relativelocation) (.z _relativelocation)) (Variables|/Script/Engine.SceneComponent|GetRelativeRotation _door_rotation_sm) false false 1.0 false)
    (else
      (Components|MoveComponentTo _door_rotation_sm_2 (Variables|/Script/Engine.SceneComponent|GetRelativeLocation _door_rotation_sm_2) (Math|Rotator|MakeRotator 0.0 0.0 (Variables|Default|Getrotation_angle)) false false 1.0 false)))
  (Input|DisableInput (Game|GetPlayerController 0))
  (Widget|RemovefromParent (stale OnComponentBeginOverlap(Box) _returnvalue_2)))

(fn ConstructionScript)