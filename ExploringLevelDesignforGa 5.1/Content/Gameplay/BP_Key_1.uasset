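; BP_Key_1 is a key pickup that grants the player character a key when collected with the Interact input.
; Overlapping its box as Ue4ASP_Character enables input and shows the W_Input prompt until the key has been taken; ending overlap disables input and removes the prompt.
; Pressing Interact sets HasKey on the character, swaps the prompt for the W_Has_key widget and destroys the actor.
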(event OnComponentBeginOverlap(Box1)
  (params (OverlappedComponent :type Primitive%20Component%20Object%20Reference) (OtherActor :type Actor%20Object%20Reference) (OtherComp :type Primitive%20Component%20Object%20Reference) (OtherBodyIndex :type Integer) (bFromSweep :type Boolean) (SweepResult :type Hit%20Result%20Structure%20%28by%20ref%29))
  (bind _returnvalue (Game|GetPlayerController 0))
  (bind _asue_4asp_character (Utilities|Casting|CastToUe4ASP_Character OtherActor))
  (if (not (Variables|Default|Getopen))
    (Input|EnableInput _returnvalue)
    (bind _returnvalue_2 (UserInterface|CreateWidget "/Game/Gameplay/W_Input.W_Input_C" _returnvalue))
    (UserInterface|Viewport|AddtoViewport _returnvalue_2 0)))

(event OnComponentEndOverlap(Box1)
  (params (OverlappedComponent :type Primitive%20Component%20Object%20Reference) (OtherActor :type Actor%20Object%20Reference) (OtherComp :type Primitive%20Component%20Object%20Reference) (OtherBodyIndex :type Integer))
  (Input|DisableInput (Game|GetPlayerController 0))
  (Widget|RemovefromParent (stale OnComponentBeginOverlap(Box1) _returnvalue_2)))

(event Input|ActionEvents|InputActionInteract
  (params (Key :type Key%20Structure :default "None"))
  (:Pressed
    (Variables|Default|Setopen true)
    (Variables|/Game/AnimStarterPack/Ue4ASP_Character.Ue4ASP_Character_C|Sethas%20key (stale OnComponentBeginOverlap(Box1) _asue_4asp_character) true)
    (bind _returnvalue (UserInterface|CreateWidget "/Game/Gameplay/W_Has_key.W_Has_key_C" (Game|GetPlayerController 0)))
    (UserInterface|Viewport|AddtoViewport _returnvalue 0)
    (Widget|RemovefromParent (stale OnComponentBeginOverlap(Box1) _returnvalue_2))
    (Actor|DestroyActor)))

(fn ConstructionScript)