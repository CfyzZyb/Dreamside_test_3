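; BP_Conveyor_01 is a conveyor Blueprint that animates a looping movement of its container component.
; BeginPlay stores the container's relative start location, then each Tick shifts it along local X by MoveRate and increments a counter.
; When the counter reaches MoveLenght, it resets and the container snaps back to the start.
; Motion counts frames without using delta time, so speed depends on frame rate.
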(event EventBeginPlay
  (bind _conveyor_contanier (Variables|Default|GetConveyor_contanier))
  (bind _relativelocation (Variables|/Script/Engine.SceneComponent|GetRelativeLocation _conveyor_contanier))
  (Variables|Default|Setstart%20postion (Math|Vector|MakeVector (.x _relativelocation) (.y _relativelocation) (.z _relativelocation))))

(event EventTick
  (params (DeltaSeconds :type Float%20%28single-precision%29))
  (bind _conveyor_contanier (Variables|Default|GetConveyor_contanier))
  (bind _relativelocation (Variables|/Script/Engine.SceneComponent|GetRelativeLocation _conveyor_contanier))
  (if (>= (Variables|Default|Getcounter) (Variables|Default|Getmove%20lenght%20))
    (Variables|Default|Setcounter 0.0)
    (Transformation|SetRelativeLocation (Variables|Default|GetConveyor_contanier) (Variables|Default|Getstart%20postion) false false)
    (else
      (Transformation|SetRelativeLocation _conveyor_contanier (Math|Vector|MakeVector (+ (.x _relativelocation) (Variables|Default|Getmove%20rate)) (.y _relativelocation) (.z _relativelocation)) false false)
      (Math|Float|IncrementFloat (Variables|Default|Getcounter)))))

(fn ConstructionScript)