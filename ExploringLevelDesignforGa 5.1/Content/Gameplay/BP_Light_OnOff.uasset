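; BP_Light_OnOff is a trigger actor that switches a skylight and a group of lights on or off on overlap.
; The Onoff flag decides whether Trigger restores the default skylight intensity and shows LightContanier, or zeroes and hides them, while Trigger_2 always restores them.
; The construction script shows the matching On or Off component, and BeginPlay resets the skylight and hides TextContanier.
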(event OnComponentBeginOverlap(Trigger)
  (params (OverlappedComponent :type Primitive%20Component%20Object%20Reference) (OtherActor :type Actor%20Object%20Reference) (OtherComp :type Primitive%20Component%20Object%20Reference) (OtherBodyIndex :type Integer) (bFromSweep :type Boolean) (SweepResult :type Hit%20Result%20Structure%20%28by%20ref%29))
  (if (Variables|Default|Geton\off)
    (Rendering|Components|Light|SetIntensity (Variables|/Script/Engine.SkyLight|GetLightComponent (Variables|Default|GetSkylight)) (Variables|Default|Getdefault_skylight))
    (Rendering|SetVisibility (Variables|Default|GetLight_contanier) true true)
    (else
      (Rendering|Components|Light|SetIntensity (Variables|/Script/Engine.SkyLight|GetLightComponent (Variables|Default|GetSkylight)) 0.0)
      (Rendering|SetVisibility (Variables|Default|GetLight_contanier) false true))))

(event OnComponentBeginOverlap(Trigger_2)
  (params (OverlappedComponent :type Primitive%20Component%20Object%20Reference) (OtherActor :type Actor%20Object%20Reference) (OtherComp :type Primitive%20Component%20Object%20Reference) (OtherBodyIndex :type Integer) (bFromSweep :type Boolean) (SweepResult :type Hit%20Result%20Structure%20%28by%20ref%29))
  (Rendering|Components|Light|SetIntensity (Variables|/Script/Engine.SkyLight|GetLightComponent (Variables|Default|GetSkylight)) (Variables|Default|Getdefault_skylight))
  (Rendering|SetVisibility (Variables|Default|GetLight_contanier) true true))

(event EventBeginPlay
  (Rendering|Components|Light|SetIntensity (Variables|/Script/Engine.SkyLight|GetLightComponent (Variables|Default|GetSkylight)) (Variables|Default|Getdefault_skylight))
  (Rendering|SetVisibility (Variables|Default|GetText_contanier) false true))

(fn ConstructionScript
  (if (Variables|Default|Geton\off)
    (Rendering|SetVisibility (Variables|Default|GetOff) false false)
    (else
      (Rendering|SetVisibility (Variables|Default|GetOn) false false))))